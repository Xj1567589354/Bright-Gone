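; Zombie enemy character that wanders, chases and attacks the player, ragdolling with a kill popup on death.
; Custom events switch speed and rotation between wander and chase.
; A forward trace each tick drives the anim Attack flag, gating Sphere overlap damage, and clears the blackboard sight key after the player dies.
; Bullet hits turn an unaware zombie toward the player, and a timeline event slides it in front of them.
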(event Custom|随机移动
  ;[0 1 0.5789 1 15] 随机移动
  (if (not (Variables|Default|Getdead))
    (Variables|/Script/Engine.CharacterMovementComponent|SetMaxWalkSpeed (Variables|Character|GetCharacterMovement) 4e+01)
    (Variables|/Script/Engine.CharacterMovementComponent|SetbOrientRotationToMovement (Variables|Character|GetCharacterMovement) true)
    (Variables|Default|SetbUseControllerRotationYaw false)))

(event Custom|发现玩家
  ;[1 0.9289 0 1 15] 发现玩家
  (if (not (Variables|Default|Getdead))
    (Variables|/Script/Engine.CharacterMovementComponent|SetMaxWalkSpeed (Variables|Character|GetCharacterMovement) 4.4e+02)
    (Variables|/Script/Engine.CharacterMovementComponent|SetbOrientRotationToMovement (Variables|Character|GetCharacterMovement) false)
    (Variables|Default|SetbUseControllerRotationYaw true)))

(event Game|Damage|EventAnyDamage
  (params (Damage :type Float%20%28single-precision%29) (DamageType :type Damage%20Type%20Object%20Reference) (InstigatedBy :type Controller%20Object%20Reference) (DamageCauser :type Actor%20Object%20Reference))
  ;[0.1804 0.02758 1 1 15] 玩家伤害敌人，敌人扣血
  (if (not (Variables|Default|Getdead))
    (bind _output_get (Variables|Default|Sethealth (- (Variables|Default|Gethealth) Damage)))
    (if (<= _output_get 0.0)
      (Physics|SetSimulatePhysics (Variables|Character|GetMesh) true)
      (Variables|Default|Setdead true)
      (Variables|/Script/Engine.CharacterMovementComponent|SetMaxWalkSpeed (Variables|Character|GetCharacterMovement) 0.0)
      (Collision|SetCollisionEnabled (Variables|Collision|GetCapsuleComponent) "NoCollision") ; 关闭碰撞
      (bind _returnvalue (UserInterface|CreateWidget "/Game/Zombies/BluePrints/KilledPopup.KilledPopup_C")) ; 击杀提示
      (UserInterface|Viewport|AddtoViewport _returnvalue 0))))

(event OnComponentBeginOverlap(Sphere)
  (params (OverlappedComponent :type Primitive%20Component%20Object%20Reference) (OtherActor :type Actor%20Object%20Reference) (OtherComp :type Primitive%20Component%20Object%20Reference) (OtherBodyIndex :type Integer) (bFromSweep :type Boolean) (SweepResult :type Hit%20Result%20Structure%20%28by%20ref%29))
  ;[0 1 0.5186 1 15] 敌人伤害玩家，玩家扣血
  (if (Variables|/Game/Zombies/BluePrints/Zombie_Anim.Zombie_Anim_C|Getattack? (.AsZombie%20Anim (Utilities|Casting|CastToZombie_Anim (Components|SkeletalMesh|GetAnimInstance (Variables|Character|GetMesh)))))
    (bind _asman_bp (Utilities|Casting|CastToMan_BP OtherActor))
    (Default|TakeDamage _asman_bp 0.1)))

(event EventTick
  (params (DeltaSeconds :type Float%20%28single-precision%29))
  (bind _returnvalue (Transformation|GetActorLocation))
  (bind _mesh (Variables|Character|GetMesh))
  (bind _returnvalue_2 (Components|SkeletalMesh|GetAnimInstance _mesh))
  (bind _aszombie_anim (Utilities|Casting|CastToZombie_Anim _returnvalue_2))
  ;[0.3115 0.09023 1 1 15] 碰撞检测，敌人攻击
  (Utilities|FlowControl|Sequence
    (:then_0
      ;[1 0.08881 0.07489 1 15] 敌人检测玩家是否死亡，如果死亡，开启敌人随机移动
      (bind _asman_bp (Utilities|Casting|CastToMan_BP (Variables|Default|GetHitActor)))
      (if (Variables|/Game/Zombies/BluePrints/Man_BP.Man_BP_C|Getdead？ _asman_bp)
        (Utilities|FlowControl|Delay 4.0)
        (AI|Components|Blackboard|SetValueasBool (AI|GetBlackboard (AI|GetAIController self)) (Utilities|Name|MakeLiteralName "CanSeePlayer?") false)))
    (:then_1
      (if (not (Variables|Default|Getdead))
        (bind (_outhit _returnvalue_3) (Collision|LineTraceByChannel _returnvalue (+ _returnvalue (* (Transformation|GetActorForwardVector) 1.8e+02)) "TraceTypeQuery1" false 0 "None")) ; 射线碰撞检测
        (if _returnvalue_3
          (Utilities|Casting|CastToMan_BP (.HitActor (Collision|BreakHitResult _outhit)) ; 如果检测成功，并且对象是玩家，则将attack设置为true
            (:then
              (Variables|/Game/Zombies/BluePrints/Zombie_Anim.Zombie_Anim_C|Setattack? _aszombie_anim true))
            (:CastFailed
              (Variables|/Game/Zombies/BluePrints/Zombie_Anim.Zombie_Anim_C|Setattack? _aszombie_anim false :!label _label)))
          (else
            (goto _label)))
        (Variables|Default|SetHitActor (.HitActor (Collision|BreakHitResult _outhit)))))
    (:then_2
      (if (Variables|Default|Getdead)
        (Collision|SetCollisionEnabled (Variables|Default|GetSphere) "NoCollision")))))

(event OnComponentHit(Mesh)
  (params (HitComponent :type Primitive%20Component%20Object%20Reference) (OtherActor :type Actor%20Object%20Reference) (OtherComp :type Primitive%20Component%20Object%20Reference) (NormalImpulse :type Vector :default "0, 0, 0") (Hit :type Hit%20Result%20Structure%20%28by%20ref%29))
  ;[1 1 1 1 15] 敌人面向玩家
  (Utilities|Casting|CastToBullet_BP OtherActor)
  (if (not (ScalableFloat|GetValueasBool (AI|GetBlackboard (AI|GetAIController self)) (Utilities|Name|MakeLiteralName "CanSeePlayer?"))) ; 判断敌人是否看见玩家
    (AI|SetFocus (AI|GetAIController self) (Game|GetPlayerCharacter 0)) ; 敌人朝向玩家
    (Variables|/Script/Engine.CharacterMovementComponent|SetbOrientRotationToMovement (Variables|Character|GetCharacterMovement) false)
    (Variables|Default|SetbUseControllerRotationYaw true)))

(event Custom|瞬移功能
  (bind _returnvalue (Game|GetPlayerCharacter 0))
  ;[1 1 1 1 15] 瞬移
  (bind _新建轨道_0 (Timeline|时间轴_0 Play)
    (:Update
      (Transformation|SetActorLocation (Math|Vector|Lerp(Vector) (Transformation|GetActorLocation) (+ (Transformation|GetActorLocation _returnvalue) (* (Transformation|GetActorForwardVector _returnvalue) 4e+02)) _新建轨道_0) false false) ; 敌人瞬移到玩家面前
    )))

(fn ConstructionScript)