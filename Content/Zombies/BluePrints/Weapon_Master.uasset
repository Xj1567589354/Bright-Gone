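; Master weapon Blueprint that handles automatic fire and reloading for the player's Man_BP character.
; Fire starts a looping timer at the weapon's fire rate if EnableFire is set, and StopFire or an empty clip clears it.
; Each shot spawns Bullet_BP from the camera, with muzzle effect, shell ejection, recoil and shake only for weapon 0.
; Reload refills the clip from reserve ammo and sets IsReload, which blocks shooting.
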(event Custom|Fire
  ;[1 0.4926 0.3907 1 15] 开火
  (bind _outactors (Actor|GetAllActorsOfClass "/Game/Zombies/BluePrints/Man_BP.Man_BP_C"))
  (if (Variables|/Game/Zombies/BluePrints/Man_BP.Man_BP_C|GetenableFire (Utilities|Array|Get(acopy) _outactors)) ; 瞄准时才能开火
    (bind _returnvalue (Utilities|Time|SetTimerbyEvent (delegate Custom|Shooting) (Variables|Default|GetShootingVelocity) true)) ; 根据射速循环执行射击事件
  ))

(event Custom|Shooting
  (bind _returnvalue (Game|GetPlayerCameraManager 0))
  (bind _arrow (Variables|Default|GetArrow))
  (bind _returnvalue_2 (Transformation|GetWorldTransform _arrow))
  ;[1 0.4926 0.3907 1 15] 开火
  (bind _asman_bp (Utilities|Casting|CastToMan_BP (Game|GetPlayerCharacter 0)))
  (if (not (Variables|/Game/Zombies/BluePrints/Man_BP.Man_BP_C|GetisReload _asman_bp))
    (if (== 0 (Variables|Default|GetBulletNum)) ; 修复子弹数量不能是负数
      (Variables|Default|SetBulletNum 0) ; 子弹为0
      ;;[1 0.9377 0.07722 1 15] 停止开火
      (Utilities|Time|ClearandInvalidateTimerbyHandle (stale Custom|Fire _returnvalue) :!label _label) ; 清除事件定时器
      (Components|Activation|SetActive (Variables|Default|GetRifle_Tracer) false true) ; 禁用枪火
      (else
        (bind _output_get (Variables|Default|SetBulletNum (- (Variables|Default|GetBulletNum) 1))) ; 子弹减1
        (if (> _output_get 0) ; 判断是否还有子弹
          (Game|SpawnActorfromClass "/Game/Zombies/BluePrints/Bullet_BP.Bullet_BP_C" (Math|Transform|MakeTransform (Camera|GetCameraLocation _returnvalue) (Camera|GetCameraRotation _returnvalue) "0.200000,0.200000,0.200000") "AdjustIfPossibleButAlwaysSpawn" 0 0) ; 在屏幕中央生成子弹
          (switch int (Variables|/Game/Zombies/BluePrints/Man_BP.Man_BP_C|GetSelectWeaNum _asman_bp)
            (:0
              (Components|Activation|SetActive (Variables|Default|GetRifle_Tracer) true true) ; 激活枪火
              (Effects|SpawnEmitteratLocation 0 (.location _returnvalue_2) (.rotation _returnvalue_2)) ; 抛弹壳
              ;;[1 0.05419 0.5317 1 15] 添加M4A1后座力
              (Class|PlayerController|AddPitchInput (Game|GetPlayerController 0) -0.3)
              (Class|PlayerCameraManager|PlayCameraShake (Game|GetPlayerCameraManager 0) "/Script/Engine.CameraShake" 0.2 "CameraLocal" "0, 0, 0")))
          (else
            (goto _label)))))))

(event Custom|StopFire
  ;[1 0.4926 0.3907 1 15] 开火
  ;;[1 0.9377 0.07722 1 15] 停止开火
  (Utilities|Time|ClearandInvalidateTimerbyHandle (stale Custom|Fire _returnvalue)) ; 清除事件定时器
  (Components|Activation|SetActive (Variables|Default|GetRifle_Tracer) false true) ; 禁用枪火
)

(fn ConstructionScript)

(fn Reload
  ;[1 1 1 1 15] 换弹
  (if (== (Variables|Default|GetBulletNum) (Variables|Default|GetBulletClipSize)) ; 判读昂当前弹夹子弹数是否等于换弹弹夹子弹数
    (Development|PrintString "子弹充足！" true true "(R=1.000000,G=0.946723,B=0.000000,A=1.000000)" 1.0)
    (Variables|Default|SetisEnough true)
    (else
      (Variables|Default|SetisEnough false)
      (if (>= (Variables|Default|GetMaxBulletNum) (Variables|Default|GetBulletClipSize)) ; 判断最大弹夹容量是否大于换弹弹夹子弹数
        (Variables|Default|SetMaxBulletNum (- (Variables|Default|GetMaxBulletNum) (- (Variables|Default|GetBulletClipSize) (Variables|Default|GetBulletNum))))
        (Variables|Default|SetBulletNum (+ (Variables|Default|GetBulletNum) (- (Variables|Default|GetBulletClipSize) (Variables|Default|GetBulletNum))))
        (bind _asman_bp (Utilities|Casting|CastToMan_BP (Game|GetPlayerCharacter 0)))
        (bind _output_get (Variables|Default|SetPlayer _asman_bp))
        (bind _output_get_2 (Variables|/Game/Zombies/BluePrints/Man_BP.Man_BP_C|SetisReload _output_get true))
        (elif (<= (- (Variables|Default|GetMaxBulletNum) (- (Variables|Default|GetBulletClipSize) (Variables|Default|GetBulletNum))) 0) ; 判断最大弹夹容量是否小于等于0
          (Variables|Default|SetBulletNum (+ (Variables|Default|GetMaxBulletNum) (Variables|Default|GetBulletNum)))
          (Variables|Default|SetMaxBulletNum 0)
          (bind _output_get_3 (Variables|/Game/Zombies/BluePrints/Man_BP.Man_BP_C|SetisReload (Variables|Default|GetPlayer) true))
          (else
            (Variables|Default|SetMaxBulletNum (- (Variables|Default|GetMaxBulletNum) (- (Variables|Default|GetBulletClipSize) (Variables|Default|GetBulletNum))))
            (Variables|Default|SetBulletNum (+ (Variables|Default|GetBulletNum) (- (Variables|Default|GetBulletClipSize) (Variables|Default|GetBulletNum))))
            (bind _output_get_4 (Variables|/Game/Zombies/BluePrints/Man_BP.Man_BP_C|SetisReload (Variables|Default|GetPlayer) true)))))
      (return _output_get_2 _output_get_3 _output_get_4))))