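; Smoke grenade actor that launches itself along the first player's view direction and releases a smoke cloud after a short fuse.
; On BeginPlay it applies a physics impulse to its static mesh using the forward vector of player controller 0's control rotation.
; After a delay, it spawns an enlarged smoke particle emitter at the mesh's current location and stores the reference.
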(event EventBeginPlay
  (Physics|AddImpulse (Variables|Default|GetStaticMesh) (* "1000.000000,1000.000000,1000.000000" (Math|Rotator|GetRotationXVector (Pawn|GetControlRotation (Game|GetPlayerController 0) :!class /Script/Engine.Controller))) "None" false) ; 添加冲量
  (Utilities|FlowControl|Delay 1.5)
  (bind _returnvalue (Effects|SpawnEmitteratLocation "/Game/StarterContent/Particles/P_Smoke.P_Smoke" (Transformation|GetWorldLocation (Variables|Default|GetStaticMesh)) "0, 0, 0" "5.000000,5.000000,5.000000")) ; 烟雾发射器
  (Variables|Default|SetSmokeEmitter _returnvalue))

(fn ConstructionScript)