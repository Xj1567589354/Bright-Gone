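; Thrown grenade actor that explodes on a short timer and damages nearby zombies.
; On BeginPlay it applies an impulse to its static mesh along the first player's control rotation.
; After a delay it attaches explosion particles and sound to the mesh, then applies damage to each Zombie_BP overlapping its Sphere component.
; The graph never destroys the actor after detonation.
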(event EventBeginPlay
  (Physics|AddImpulse (Variables|Default|GetStaticMesh) (* "1000.000000,1000.000000,1000.000000" (Math|Rotator|GetRotationXVector (Pawn|GetControlRotation (Game|GetPlayerController 0) :!class /Script/Engine.Controller))) "None" false) ; 添加冲量
  (Utilities|FlowControl|Delay 1.5)
  (Effects|SpawnEmitterAttached "/Game/Weapons/MilitaryWeapSilver/FX/P_Grenade_Explosion_01.P_Grenade_Explosion_01" (Variables|Default|GetStaticMesh) "None" "0, 0, 0" "0, 0, 0" "15.000000,15.000000,15.000000") ; 手雷爆炸效果
  (Audio|SpawnSoundAttached "/Game/Weapons/MilitaryWeapSilver/Sound/GrenadeLauncher/Wavs/GrenadeLauncher_Explosion03.GrenadeLauncher_Explosion03" (Variables|Default|GetStaticMesh) "None" "0, 0, 0" "0, 0, 0" "KeepRelativeOffset" false 1.0 1.0 0.0 0 0) ; 手雷爆炸声效
  (for _array_element (Collision|GetOverlappingActors (Variables|Default|GetSphere) "/Game/Zombies/BluePrints/Zombie_BP.Zombie_BP_C" :!class /Script/Engine.PrimitiveComponent)
    (bind _aszombie_bp (Utilities|Casting|CastToZombie_BP _array_element))
    (Game|Damage|ApplyDamage _aszombie_bp 0.5 0 0)))

(fn ConstructionScript)