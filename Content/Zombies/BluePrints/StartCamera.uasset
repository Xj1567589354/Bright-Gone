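; StartCamera is an intro camera actor that hands the view and control over to the player character.
; While IOState is true, Tick waits on a Delay, then finds the first Man_BP actor.
; It blends player controller 0's view to that actor, waits out the blend, possesses it and destroys itself.
; The sequence runs from Tick through latent Delays, and IOState is not set in this graph.
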(event EventTick
  (params (DeltaSeconds :type Float%20%28single-precision%29))
  (bind _returnvalue (Game|GetPlayerController 0))
  ;[1 0.7685 0.02322 1 15] 镜头过渡
  (if (Variables|Default|GetIOState)
    (Utilities|FlowControl|Delay 6.0) ; 镜头停留5s
    (bind _outactors (Actor|GetAllActorsOfClass "/Game/Zombies/BluePrints/Man_BP.Man_BP_C"))
    (bind _output_get (Variables|Default|SetPlayer (Utilities|Array|Get(acopy) _outactors)))
    (Game|Player|SetViewTargetwithBlend _returnvalue _output_get 3.0 "VTBlend_Linear" 0.0 false) ; 镜头过渡3s
    (Utilities|FlowControl|Delay 3.0)
    (Pawn|Possess _returnvalue (Variables|Default|GetPlayer)) ; 切换控制权
    (Actor|DestroyActor)))

(fn ConstructionScript)