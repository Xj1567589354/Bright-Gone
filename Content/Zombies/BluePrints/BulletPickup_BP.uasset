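; Ammo pickup actor that refills the weapon the player character (Man_BP) has selected when it enters the sphere trigger.
; SelectWeaNum picks the M4A1 or AK47, whose MaxBulletNum rises by a fixed amount, clamped to a per-weapon cap.
; Either branch then sets the character's IsPickUpArmor flag, adds a Pickup widget to the viewport and destroys the actor.
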(event OnComponentBeginOverlap(Sphere)
  (params (OverlappedComponent :type Primitive%20Component%20Object%20Reference) (OtherActor :type Actor%20Object%20Reference) (OtherComp :type Primitive%20Component%20Object%20Reference) (OtherBodyIndex :type Integer) (bFromSweep :type Boolean) (SweepResult :type Hit%20Result%20Structure%20%28by%20ref%29))
  ;[0.6576 0.3312 1 1 15] 补充弹夹
  (bind _asman_bp (Utilities|Casting|CastToMan_BP OtherActor))
  (Variables|Default|SetMan _asman_bp)
  (Variables|Default|SetWeapon%20M4A1 (Variables|/Game/Zombies/BluePrints/Man_BP.Man_BP_C|GetWeapon_M4A1 _asman_bp))
  (Variables|Default|SetWeapon%20AK47 (Variables|/Game/Zombies/BluePrints/Man_BP.Man_BP_C|GetWeapon%20AK47 _asman_bp))
  (switch int (Variables|/Game/Zombies/BluePrints/Man_BP.Man_BP_C|GetSelectWeaNum _asman_bp)
    (:0
      (if (>= (+ (Variables|/Game/Zombies/BluePrints/Weapon_Master.Weapon_Master_C|GetMaxBulletNum (Variables|Default|GetWeapon%20M4A1)) 50) 120) ; 判断弹夹容量是否最大值
        (Variables|/Game/Zombies/BluePrints/Weapon_Master.Weapon_Master_C|SetMaxBulletNum (Variables|Default|GetWeapon%20M4A1) 120)
        (else
          (Variables|/Game/Zombies/BluePrints/Weapon_Master.Weapon_Master_C|SetMaxBulletNum (Variables|Default|GetWeapon%20M4A1) (+ (Variables|/Game/Zombies/BluePrints/Weapon_Master.Weapon_Master_C|GetMaxBulletNum (Variables|Default|GetWeapon%20M4A1)) 50))))
      (Variables|/Game/Zombies/BluePrints/Man_BP.Man_BP_C|SetisPickUpArmor? (Variables|Default|GetMan) true)
      (bind _returnvalue (UserInterface|CreateWidget "/Game/Zombies/BluePrints/Pickup.Pickup_C")) ; 拾取信息
      (UserInterface|Viewport|AddtoViewport _returnvalue 0)
      (Actor|DestroyActor))
    (:1
      (if (>= (+ (Variables|/Game/Zombies/BluePrints/Weapon_AK47.Weapon_AK47_C|GetMaxBulletNum (Variables|Default|GetWeapon%20AK47)) 50) 150) ; 判断弹夹容量是否最大值
        (Variables|/Game/Zombies/BluePrints/Weapon_AK47.Weapon_AK47_C|SetMaxBulletNum (Variables|Default|GetWeapon%20AK47) 150)
        (else
          (Variables|/Game/Zombies/BluePrints/Weapon_AK47.Weapon_AK47_C|SetMaxBulletNum (Variables|Default|GetWeapon%20AK47) (+ (Variables|/Game/Zombies/BluePrints/Weapon_AK47.Weapon_AK47_C|GetMaxBulletNum (Variables|Default|GetWeapon%20AK47)) 50))))
      (Variables|/Game/Zombies/BluePrints/Man_BP.Man_BP_C|SetisPickUpArmor? (Variables|Default|GetMan) true)
      (bind _returnvalue_2 (UserInterface|CreateWidget "/Game/Zombies/BluePrints/Pickup.Pickup_C")) ; 拾取信息
      (UserInterface|Viewport|AddtoViewport _returnvalue_2 0)
      (Actor|DestroyActor))))

(event EventBeginPlay)

(event Collision|EventActorBeginOverlap
  (params (OtherActor :type Actor%20Object%20Reference)))

(event EventTick
  (params (DeltaSeconds :type Float%20%28single-precision%29))
  ;[0.6576 0.3312 1 1 15] 补充弹夹
)

(fn ConstructionScript)