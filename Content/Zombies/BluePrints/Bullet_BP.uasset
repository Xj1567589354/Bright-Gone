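; Bullet projectile for the zombie shooter that plays the firing sound and resolves impacts.
; BeginPlay picks the gunshot sound from the player Man_BP's AK47 selection flag.
; Hits damage zombies with a blood effect and hit-marker widget; other surfaces get stone sparks and a bullet-hole decal.
; It then pushes physics-simulating components and destroys itself, except when the zombie is already dead after damage.
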(event EventBeginPlay
  ;[1 1 1 1 15] 子弹音效
  (bind _asman_bp (Utilities|Casting|CastToMan_BP (Game|GetPlayerCharacter 0)))
  (if (Variables|/Game/Zombies/BluePrints/Man_BP.Man_BP_C|GetisSelectAK47 _asman_bp)
    (Audio|PlaySoundatLocation "/Game/Weapons/AK47-2/Assault_Rifle_Shot_03.Assault_Rifle_Shot_03" (Transformation|GetActorLocation) "0, 0, 0" 1.0 1.0 0.0 0 0 0)
    (else
      (Audio|PlaySoundatLocation "/Game/Weapons/MilitaryWeapSilver/Sound/Rifle/Wavs/RifleA_Fire_ST01.RifleA_Fire_ST01" (Transformation|GetActorLocation) "0, 0, 0" 1.0 1.0 0.0 0 0 0))))

(event Collision|EventHit
  (params (MyComp :type Primitive%20Component%20Object%20Reference) (Other :type Actor%20Object%20Reference) (OtherComp :type Primitive%20Component%20Object%20Reference) (bSelfMoved :type Boolean) (HitLocation :type Vector :default "0, 0, 0") (HitNormal :type Vector :default "0, 0, 0") (NormalImpulse :type Vector :default "0, 0, 0") (Hit :type Hit%20Result%20Structure%20%28by%20ref%29))
  (bind _returnvalue (Math|Rotator|MakeRotfromX HitNormal))
  ;[1 1 1 1 15] 子弹命中事件
  (bind _aszombie_bp (Utilities|Casting|CastToZombie_BP Other)
    (:then
      (Effects|SpawnEmitteratLocation "/Game/FXVillesBloodVFXPack/Particles/PS_StyleBlood_Slash_Omni_MED.PS_StyleBlood_Slash_Omni_MED" HitLocation _returnvalue) ; 子弹命中敌人生成发射器
      (Game|Damage|ApplyDamage _aszombie_bp 0.05 0 0)
      (if (not (Variables|/Game/Zombies/BluePrints/Zombie_BP.Zombie_BP_C|Getdead _aszombie_bp)) ; 判断当前丧尸是否已死亡
        (bind _returnvalue_2 (UserInterface|CreateWidget "/Game/Zombies/BluePrints/Hit_Zombies.Hit_Zombies_C")) ; 创建命中准星
        (UserInterface|Viewport|AddtoViewport _returnvalue_2 0)
        (if (Physics|IsSimulatingPhysics OtherComp "None") :!label _label
          (Physics|AddImpulse OtherComp (* (Transformation|GetVelocity) 0.5) "None" false) ; 命中物体，添加冲力
        )
        (Actor|DestroyActor self)))
    (:CastFailed
      (Effects|SpawnEmitteratLocation "/Game/Weapons/MilitaryWeapSilver/FX/P_Impact_Stone_Medium_01.P_Impact_Stone_Medium_01" HitLocation _returnvalue) ; 子弹命中位置生成发射器
      (Rendering|Decal|SpawnDecalatLocation "/Game/UWC_Bullet_Holes/Instances/Decals/Asphalt/MI_Asphalt_1.MI_Asphalt_1" "5.000000,5.000000,5.000000" HitLocation _returnvalue 0.0) ; 产生弹孔
      (goto _label))))

(fn ConstructionScript)