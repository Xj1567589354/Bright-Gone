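; Player character for a zombie shooter, with first/third-person views, aiming, sprint, crouch and a montage roll.
; Spawns M4A1 and AK47 on mesh sockets, switching visibility once the AK47 is picked up, and throws frag and smoke grenades.
; Tick polls state with Delays for armor regen, HUD creation, countdown and pickup text.
; Damage drains armor before health; death triggers ragdoll, death camera and UI, then quits the game.
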(event EventBeginPlay
  ;[1 0.02841 0 1 15] 角色装配M4A1
  (Utilities|FlowControl|Sequence
    (:then_0
      (bind _returnvalue (Game|SpawnActorfromClass "/Game/Zombies/BluePrints/Weapon_Master.Weapon_Master_C" (Math|Transform|MakeTransform "0, 0, 0") "Undefined" 0 0)) ; 系统运行时生成M4A1
      (bind _output_get (Variables|Default|SetWeapon_M4A1 _returnvalue))
      (Transformation|AttachComponentToComponent _output_get (Variables|Character|GetMesh) "Weapon_Socket_M4A1" "SnapToTarget" "SnapToTarget" "SnapToTarget" true) ; 将M4A1附着在角色身上
      (bind _returnvalue_2 (Game|SpawnActorfromClass "/Game/Zombies/BluePrints/Weapon_AK47.Weapon_AK47_C" (Math|Transform|MakeTransform "0, 0, 0") "Undefined" 0 0)) ; 系统运行时生成AK47
      (bind _output_get_2 (Variables|Default|SetWeapon%20AK47 _returnvalue_2))
      (Transformation|AttachComponentToComponent _output_get_2 (Variables|Character|GetMesh) "Weapon_Socket_AK47" "SnapToTarget" "SnapToTarget" "SnapToTarget" true) ; 将M4A1附着在角色身上
      (Rendering|SetVisibility (Variables|/Game/Zombies/BluePrints/Weapon_AK47.Weapon_AK47_C|GetSkeletalMesh (Variables|Default|GetWeapon%20AK47)) false false))
    (:then_1
      (bind _asman_anim_more (Utilities|Casting|CastToMan_Anim_More (Components|SkeletalMesh|GetAnimInstance (Variables|Character|GetMesh))))
      (Variables|Default|SetManAnimMore _asman_anim_more))))

(event EventTick
  (params (DeltaSeconds :type Float%20%28single-precision%29))
  (Utilities|FlowControl|Sequence
    (:then_0
      ;[0 1 0.05444 1 15] 角色速度判断
      (bind _returnvalue (CallFunction|角色速度判断))
      (Variables|/Script/Engine.CharacterMovementComponent|SetMaxWalkSpeed (Variables|Character|GetCharacterMovement) _returnvalue))
    (:then_1
      ;[0.05855 0.7063 1 1 15] 玩家死亡之后，停止开火
      (if (Variables|Default|Getdead？)
        (Default|StopFire (Variables|Default|GetWeapon_M4A1))))
    (:then_2
      (CallFunction|角色死亡判断) ; 镜头过渡
    )
    (:then_3
      ;[0.6652 1 0.7334 1 15] 盔甲值自动恢复0.01
      (if (not (Variables|Default|Getdead？))
        (if (not (Variables|Default|GetisDamage)) ; 判断是否受到伤害
          (Utilities|FlowControl|Delay 1.5)
          (if (< (Variables|Default|Getarmor) 0.99) ; 判断盔甲值是否是满值
            (Variables|Default|Setarmor (+ (Variables|Default|Getarmor) 0.01))))))
    (:then_4
      ;[0 1 0.6441 1 15] 设置死亡状态，创建死亡UI
      (CallFunction|死亡))
    (:then_5
      ;[1 0.2321 0.1544 1 15] 销毁HUD
      (if (Variables|Default|GetisHud) ; 判断是否创建HUD
        (if (Variables|Default|Getdead？) ; 判断是否死亡
          (Widget|RemovefromParent (Variables|Default|GetHUD))
          (Variables|Default|SetHUD 0)
          (Variables|Default|SetisHud false))))
    (:then_6
      (if (Variables|Default|GetisStartMenu) ; 判断是否开始游戏
        (Utilities|FlowControl|Delay 1e+01)
        ;[1 0 0.2972 1 15] 创建HUD
        (bind _returnvalue_2 (UserInterface|CreateWidget "/Game/Zombies/BluePrints/HUD.HUD_C"))
        (bind _output_get (Variables|Default|SetHUD _returnvalue_2))
        (UserInterface|Viewport|AddtoViewport _output_get 0)
        (Variables|Default|SetisHud true)
        (Variables|Default|SetisStartMenu false)
        (Utilities|FlowControl|Delay 1.0)
        (Variables|Default|SetisTimer true) ; 计时器状态
      ))
    (:then_7
      ;[1 0 0.9481 1 15] 计时器
      (if (Variables|Default|GetisTimer) ; 判断是否已开启计时器
        (Utilities|FlowControl|Delay 1.0)
        (bind _output_get_2 (Variables|Default|Setseconds (- (Variables|Default|Getseconds) 1)))
        (if (<= _output_get_2 0) ; 判断秒钟是否小于0
          (Variables|Default|Setseconds 59)
          (bind _output_get_3 (Variables|Default|Setminutes (- (Variables|Default|Getminutes) 1)))
          (if (or (== _output_get_3 0) (Variables|Default|Getdead？)) ; 判断分钟是否等于0或者玩家是否死亡
            (Variables|Default|SetisTimer false)))))
    (:then_8
      ;[0.9225 1 0 1 15] 拾取信息修改
      (if (Variables|Default|GetisPickupAK47?)
        (if (Variables|Default|GetisEnableAK47State)
          (Variables|Default|SetisPickUpText "拾取一把AK47")
          (Utilities|FlowControl|Delay 2.0)
          (Variables|Default|SetisEnableAK47State false))))
    (:then_9
      (if (Variables|Default|GetisPickUpArmor?)
        (Variables|Default|SetisPickUpText "拾取一匣弹夹")
        (Utilities|FlowControl|Delay 2.0)
        (Variables|Default|SetisPickUpArmor? false)))
    (:then_10
      ;[0.3041 0.9262 1 1 15] 手雷提示
      (Utilities|FlowControl|Sequence
        (:then_0
          (if (Variables|Default|GetisPickFlagGrenate)
            (Variables|Default|SetisPickUpText "拾取两颗手雷")
            (Utilities|FlowControl|Delay 2.0)
            (Variables|Default|SetisPickFlagGrenate false)))
        (:then_1
          (if (Variables|Default|GetisPickSmokeGrenate)
            (Variables|Default|SetisPickUpText "拾取两颗烟雾弹")
            (Utilities|FlowControl|Delay 2.0)
            (Variables|Default|SetisPickSmokeGrenate false)))))))

(event Input|ActionEvents|InputActionCrouch
  (params (Key :type Key%20Structure))
  (bind _charactermovement (Variables|Character|GetCharacterMovement))
  ;[1 0.7859 0.7155 1 15] 按Ctrl实现蹲伏
  (:Pressed
    (if (Variables|Default|Getrun?) ; 判断奔跑状态
      (Variables|Default|Setrun? false))
    (Variables|Default|SetisCrouch true)
    (Variables|/Script/Engine.CharacterMovementComponent|SetMaxWalkSpeed _charactermovement 3e+02)
    (Character|Crouch))
  (:Released
    (Variables|Default|SetisCrouch false)
    (Variables|/Script/Engine.CharacterMovementComponent|SetMaxWalkSpeed _charactermovement 6e+02)
    (Character|UnCrouch)))

(event Input|AxisEvents|InputAxisMoveForward
  (params (AxisValue :type Float%20%28single-precision%29))
  ;[0.07394 0 1 1 15] 控制玩家移动
  (Pawn|Input|AddMovementInput (Math|Vector|GetForwardVector (Math|Rotator|MakeRotator 0.0 0.0 (.yaw (Pawn|GetControlRotation :!class /Script/Engine.Pawn)))) AxisValue false))

(event Input|AxisEvents|InputAxisMoveRight
  (params (AxisValue :type Float%20%28single-precision%29))
  ;[0.07394 0 1 1 15] 控制玩家移动
  (Pawn|Input|AddMovementInput (Math|Vector|GetRightVector (Math|Rotator|MakeRotator 0.0 0.0 (.yaw (Pawn|GetControlRotation :!class /Script/Engine.Pawn)))) AxisValue false))

(event Input|AxisEvents|InputAxisTurn
  (params (AxisValue :type Float%20%28single-precision%29))
  ;[1 0.01152 0 1 15] 控制摄像机视角
  (Pawn|Input|AddControllerYawInput AxisValue))

(event Input|AxisEvents|InputAxisLookUp
  (params (AxisValue :type Float%20%28single-precision%29))
  ;[1 0.01152 0 1 15] 控制摄像机视角
  (Pawn|Input|AddControllerPitchInput AxisValue))

(event Input|KeyboardEvents|LeftShift
  (params (Key :type Key%20Structure))
  ;[1 0 0.722 1 15] 按Shift键实现奔跑
  (:Pressed
    (if (Variables|Default|GetisCrouch)
      (Variables|Default|SetisCrouch false) ; 判断蹲伏状态
      (Character|Crouch))
    (Variables|Default|Setrun? true))
  (:Released
    (Variables|Default|Setrun? false)))

(event Input|KeyboardEvents|SpaceBar
  (params (Key :type Key%20Structure))
  (bind _mesh (Variables|Character|GetMesh))
  (bind _returnvalue (Components|SkeletalMesh|GetAnimInstance _mesh))
  ;[0 1 0.3589 1 15] 按空格键实现跳跃
  (:Pressed
    (if (not (Animation|Montage|MontageIsPlaying _returnvalue "/Game/Zombies/models/Man/Animations/ManRollForward_Root_Anim_Montage.ManRollForward_Root_Anim_Montage")) ; 判断动画是否在播放
      (Animation|Montage|MontagePlay _returnvalue "/Game/Zombies/models/Man/Animations/ManRollForward_Root_Anim_Montage.ManRollForward_Root_Anim_Montage" 1.0 "MontageLength" 0.0 true))))

(event Input|KeyboardEvents|V
  (params (Key :type Key%20Structure))
  (bind _mananimmore (Variables|Default|GetManAnimMore))
  (bind _firstcamera (Variables|Default|GetFirstCamera))
  (bind _thirdcamera (Variables|Default|GetThirdCamera))
  ;[0.02389 0.8219 1 1 15] 按V键实现第一人称和第三人称切换
  (:Pressed
    (Utilities|FlowControl|FlipFlop
      (:A
        (Components|Activation|SetActive _firstcamera true false)
        (Components|Activation|SetActive _thirdcamera false false)
        (Variables|/Game/Zombies/BluePrints/Man_Anim_More.Man_Anim_More_C|Setaim？ _mananimmore true)
        ;;[1 0.6442 0.01089 1 15] 添加准星
        (bind _returnvalue (UserInterface|CreateWidget "/Game/Zombies/BluePrints/Sight_Bead.Sight_Bead_C"))
        (UserInterface|Viewport|AddtoViewport _returnvalue 0)
        ;;[0 0.6333 1 1 15] 镜头跟随鼠标移动
        (Variables|/Script/Engine.CharacterMovementComponent|SetbOrientRotationToMovement (Variables|Character|GetCharacterMovement) false)
        (Variables|Default|SetbUseControllerRotationYaw true)
        (Variables|Default|SetenableFirstView true) ; 开启第一人称
        (Variables|Default|SetenableFire true))
      (:B
        (Components|Activation|SetActive _firstcamera false false)
        (Components|Activation|SetActive _thirdcamera true false)
        (Variables|/Game/Zombies/BluePrints/Man_Anim_More.Man_Anim_More_C|Setaim？ _mananimmore false)
        ;;[1 0.48 0.9448 1 15] 清除准星
        (Widget|RemovefromParent _returnvalue)
        (Variables|Default|SetSightBead 0)
        ;;[0.006896 1 0.3468 1 15] 镜头跟随玩家旋转移动
        (Variables|/Script/Engine.CharacterMovementComponent|SetbOrientRotationToMovement (Variables|Character|GetCharacterMovement) true)
        (Variables|Default|SetbUseControllerRotationYaw false)
        (Variables|Default|SetenableFirstView false) ; 关闭第一人称
        (Variables|Default|SetenableFire false) ; 启用开火
      ))))

(event Input|MouseEvents|RightMouseButton
  (params (Key :type Key%20Structure))
  (bind _charactermovement (Variables|Character|GetCharacterMovement))
  (bind _dead_ (Variables|Default|Getdead？))
  (bind _enablefirstview (Variables|Default|GetenableFirstView))
  ;[1 1 1 1 15] 鼠标右键实现瞄准功能
  (:Pressed
    (if (not _enablefirstview) ; 判断是否开启第一人称
      (Variables|Default|SetenableFire true)
      (if (not _dead_)
        (Variables|Default|Setaiming? true) ; 设置瞄准时角色速度
        (Variables|Default|SetEnableHUD true)
        (Variables|/Game/Zombies/BluePrints/Man_Anim_More.Man_Anim_More_C|Setaim？ (Variables|Default|GetManAnimMore) true) ; 瞄准
        ;;[1 0.6442 0.01089 1 15] 添加准星
        (bind _returnvalue (UserInterface|CreateWidget "/Game/Zombies/BluePrints/Sight_Bead.Sight_Bead_C"))
        (bind _output_get (Variables|Default|SetSightBead _returnvalue))
        (UserInterface|Viewport|AddtoViewport _output_get 0)
        ;;[0 0.6333 1 1 15] 镜头跟随鼠标移动
        (Variables|/Script/Engine.CharacterMovementComponent|SetbOrientRotationToMovement _charactermovement false)
        (Variables|Default|SetbUseControllerRotationYaw true)
        (bind _新建轨道_0 (Timeline|时间轴_0 Play)
          (:Update
            (Variables|/Script/Engine.SpringArmComponent|SetTargetArmLength (Variables|Default|GetSpringArm) (Math|Float|Lerp 175.0 5e+01 _新建轨道_0)) ; 设置镜头焦距
          )))))
  (:Released
    (if (not _enablefirstview)
      (Variables|Default|SetenableFire false)
      (if (not _dead_)
        (Variables|Default|Setaiming? false)
        (Variables|Default|SetEnableHUD false)
        (Variables|/Game/Zombies/BluePrints/Man_Anim_More.Man_Anim_More_C|Setaim？ (Variables|Default|GetManAnimMore) false)
        ;;[1 0.48 0.9448 1 15] 清除准星
        (Widget|RemovefromParent (Variables|Default|GetSightBead))
        (Variables|Default|SetSightBead 0)
        ;;[0.006896 1 0.3468 1 15] 镜头跟随玩家旋转移动
        (Variables|/Script/Engine.CharacterMovementComponent|SetbOrientRotationToMovement _charactermovement true)
        (Variables|Default|SetbUseControllerRotationYaw false)
        (Timeline|时间轴_0 Reverse)))))

(event Input|MouseEvents|LeftMouseButton
  (params (Key :type Key%20Structure))
  ;[1 1 1 1 15] 鼠标左键实现开火功能
  (:Pressed
    (if (not (Variables|Default|Getdead？))
      (switch int (Variables|Default|GetSelectWeaNum) ; 判断角色当前手持哪把枪
        (:0
          (Default|Fire (Variables|Default|GetWeapon_M4A1))
          (Variables|Default|Setaiming? true) ; 瞄准
        )
        (:1
          (Default|Fire (Variables|Default|GetWeapon%20AK47))
          (Variables|Default|Setaiming? true) ; 瞄准
        ))))
  (:Released
    (switch int (Variables|Default|GetSelectWeaNum)
      (:0
        (Default|StopFire (Variables|Default|GetWeapon_M4A1))
        (Variables|Default|Setaiming? false))
      (:1
        (Default|StopFire (Variables|Default|GetWeapon%20AK47))
        (Variables|Default|Setaiming? false)))))

(event Custom|死亡UI
  ;[1 0.4655 0.1912 1 15] 死亡UI
  (Utilities|FlowControl|Delay 3.0)
  (bind _returnvalue (UserInterface|CreateWidget "/Game/Zombies/BluePrints/DeadUI.DeadUI_C"))
  (bind _output_get (Variables|Default|SetDeadUI _returnvalue))
  (UserInterface|Viewport|AddtoViewport _output_get 0)
  (Utilities|FlowControl|Sequence
    (:then_0
      (UserInterface|Animation|PlayAnimation (Variables|Default|GetDeadUI) (Variables|/Game/Zombies/BluePrints/DeadUI.DeadUI_C|GetBG_IO _output_get) 0.0 1 "Forward" 1.0 false))
    (:then_1
      (UserInterface|Animation|PlayAnimation (Variables|Default|GetDeadUI) (Variables|/Game/Zombies/BluePrints/DeadUI.DeadUI_C|GetLBG_IO _output_get) 0.0 1 "Forward" 1.0 false))))

(event Custom|角色摄像头偏移
  ;[0.1643 0.4451 1 1 15] 角色摄像头偏移
  (Components|Activation|SetActive (Variables|Default|GetDeadCamera) true false)
  (Components|Activation|SetActive (Variables|Default|GetThirdCamera) false false)
  (Components|Activation|SetActive (Variables|Default|GetFirstCamera) false false)
  (bind _新建轨道_0 (Timeline|权重 Play)
    (:Update
      (Variables|/Script/Engine.SpringArmComponent|SetTargetArmLength (Variables|Default|GetSpringArm1) (Math|Float|Lerp 2e+02 5e+02 _新建轨道_0))
      (Variables|/Script/Engine.CharacterMovementComponent|SetbOrientRotationToMovement (Variables|Character|GetCharacterMovement) false)
      (Variables|Default|SetbUseControllerRotationYaw false)
      (Variables|/Script/Engine.SpringArmComponent|SetbUsePawnControlRotation (Variables|Default|GetSpringArm1) false))))

(event Custom|死亡
  ;[0 1 0.2548 1 15] 死亡
  (if (<= (Variables|Default|Gethealth) 0.0)
    (Physics|SetSimulatePhysics (Variables|Character|GetMesh) true) ; 开启玩家物理模拟，死亡
    (Variables|Default|Setdead？ true)
    (Collision|SetCollisionEnabled (Variables|Collision|GetCapsuleComponent) "NoCollision") ; 关闭碰撞
    (CallFunction|死亡UI)
    (Utilities|FlowControl|Delay 1e+01)
    (Game|QuitGame 0 "Quit" false)))

(event Input|ActionEvents|InputActionReload
  (params (Key :type Key%20Structure))
  ;[1 0.9428 0 1 15] 按R键实现换弹
  (:Pressed
    (switch int (Variables|Default|GetSelectWeaNum)
      (:0
        (if (not (== 0 (Variables|/Game/Zombies/BluePrints/Weapon_Master.Weapon_Master_C|GetMaxBulletNum (Variables|Default|GetWeapon_M4A1)))) ; 判断是否弹夹还有子弹
          (bind (_output_get _output_get1 _output_get2) (Default|Reload (Variables|Default|GetWeapon_M4A1)))
          (if (Math|Boolean|ORBoolean _output_get _output_get1 _output_get2)
            (Utilities|FlowControl|Delay 2.2)
            (Variables|Default|SetisReload false)
            (if (not (Variables|/Game/Zombies/BluePrints/Weapon_Master.Weapon_Master_C|GetisEnough (Variables|Default|GetWeapon_M4A1)))
              (Audio|PlaySoundatLocation "/Game/Weapons/MilitaryWeapSilver/Sound/Rifle/Wavs/Rifle_Reload02.Rifle_Reload02" (Transformation|GetActorLocation) "0, 0, 0" 1.0 1.0 0.0 0 0 0)))))
      (:1
        (if (not (== 0 (Variables|/Game/Zombies/BluePrints/Weapon_AK47.Weapon_AK47_C|GetMaxBulletNum (Variables|Default|GetWeapon%20AK47)))) ; 判断是否弹夹还有子弹
          (bind (_output_get_2 _output_get1_2 _output_get2_2) (Default|Reload (Variables|Default|GetWeapon%20AK47)))
          (if (Math|Boolean|ORBoolean _output_get_2 _output_get1_2 _output_get2_2)
            (Utilities|FlowControl|Delay 2.2)
            (Variables|Default|SetisReload false)
            (if (not (Variables|/Game/Zombies/BluePrints/Weapon_AK47.Weapon_AK47_C|GetisEnough (Variables|Default|GetWeapon%20AK47)))
              (Audio|PlaySoundatLocation "/Game/Weapons/MilitaryWeapSilver/Sound/Rifle/Wavs/Rifle_Reload02.Rifle_Reload02" (Transformation|GetActorLocation) "0, 0, 0" 1.0 1.0 0.0 0 0 0))))))))

(event Input|ActionEvents|InputActionSelectPrimary
  (params (Key :type Key%20Structure))
  ;[0.2193 1 0.592 1 15] 按1键切换M4A1
  (:Pressed
    (if (not (Variables|Default|GetisReload))
      (Variables|Default|SetisSelectAK47 false)
      (Variables|Default|SetSelectWeaNum 0)
      (Rendering|SetVisibility (Variables|/Game/Zombies/BluePrints/Weapon_AK47.Weapon_AK47_C|GetSkeletalMesh (Variables|Default|GetWeapon%20AK47)) false false)
      (Rendering|SetVisibility (Variables|/Game/Zombies/BluePrints/Weapon_Master.Weapon_Master_C|GetSkeletalMesh (Variables|Default|GetWeapon_M4A1)) true false))))

(event Input|ActionEvents|InputActionSelectSecondary
  (params (Key :type Key%20Structure))
  ;[1 0.2015 0.5497 1 15] 按2键切换AK47
  (:Pressed
    (if (not (Variables|Default|GetisReload))
      (Variables|Default|SetisSelectAK47 true)
      (if (Variables|Default|GetisPickupAK47?) ; 判断角色是否持有AK47
        (Variables|Default|SetSelectWeaNum 1)
        (Rendering|SetVisibility (Variables|/Game/Zombies/BluePrints/Weapon_AK47.Weapon_AK47_C|GetSkeletalMesh (Variables|Default|GetWeapon%20AK47)) true false)
        (Rendering|SetVisibility (Variables|/Game/Zombies/BluePrints/Weapon_Master.Weapon_Master_C|GetSkeletalMesh (Variables|Default|GetWeapon_M4A1)) false false)))))

(event Input|ActionEvents|InputActionGrenade
  (params (Key :type Key%20Structure :default "None"))
  ;[1 0.1971 0.1832 1 15] 按G键扔手雷
  (:Pressed
    (if (> (Variables|Default|GetFlagGrenate) 0)
      (Utilities|FlowControl|Delay 0.5)
      (bind _returnvalue (Game|SpawnActorfromClass "/Game/Zombies/BluePrints/Grenade_BP.Grenade_BP_C" (Math|Transform|MakeTransform (+ (Transformation|GetActorLocation) (Math|Vector|RotateVector "100.000000,0.000000,0.000000" (Pawn|GetControlRotation :!class /Script/Engine.Pawn))) (Transformation|GetActorRotation)) "Undefined" 0 0))
      (Math|Integer|DecrementInt (Variables|Default|GetFlagGrenate)
        (:%20%20
          (Utilities|FlowControl|Delay 2.0)
          (Actor|DestroyActor _returnvalue))))))

(event Input|ActionEvents|InputActionSmokeGrenade
  (params (Key :type Key%20Structure :default "None"))
  ;[0.2737 0.9582 1 1 15] 按F键扔烟雾弹
  (:Pressed
    (if (> (Variables|Default|GetSmokeGrenate) 0)
      (Utilities|FlowControl|Delay 0.5)
      (bind _returnvalue (Game|SpawnActorfromClass "/Game/Zombies/BluePrints/SmokeGrenate_BP.SmokeGrenate_BP_C" (Math|Transform|MakeTransform (+ (Transformation|GetActorLocation) (Math|Vector|RotateVector "100.000000,0.000000,0.000000" (Pawn|GetControlRotation :!class /Script/Engine.Pawn))) (Transformation|GetActorRotation)) "Undefined" 0 0))
      (Math|Integer|DecrementInt (Variables|Default|GetSmokeGrenate)
        (:%20%20
          (Utilities|FlowControl|Delay 15.0)
          (Components|DestroyComponent (Variables|/Game/Zombies/BluePrints/SmokeGrenate_BP.SmokeGrenate_BP_C|GetSP _returnvalue))
          (Actor|DestroyActor _returnvalue))))))

(event Input|KeyboardEvents|Escape
  (params (Key :type Key%20Structure))
  (bind _returnvalue (Game|GetPlayerController 0))
  ;[1 1 1 1 15] 按Escape弹出副菜单
  (:Pressed
    (bind _returnvalue_2 (UserInterface|CreateWidget "/Game/Zombies/BluePrints/ViceMenu.ViceMenu_C"))
    (bind _output_get (Variables|Default|SetViceMenu_ _returnvalue_2))
    (UserInterface|Viewport|AddtoViewport _output_get 0)
    (Variables|/Script/Engine.PlayerController|SetbShowMouseCursor _returnvalue true)
    (Input|SetInputModeUIOnly _returnvalue 0 "DoNotLock")))

(fn ConstructionScript)

(fn 角色速度判断
  ;[1 1 1 1 15] 角色速度判断
  (return (Math|Float|SelectFloat 0.0 (Math|Float|SelectFloat 3e+02 (Math|Float|SelectFloat 6e+02 3e+02 (Variables|Default|Getrun?)) (Variables|Default|Getaiming?)) (Variables|Default|Getdead？))))

(fn 角色死亡判断
  (if (Variables|Default|Getdead？)
    (Utilities|FlowControl|Sequence
      (:then_0
        (CallFunction|角色摄像头偏移)))))

(fn TakeDamage
  (params (B :type Float%20%28single-precision%29))
  (bind _output_get (Variables|Default|Setarmor (- (Variables|Default|Getarmor) B)))
  (if (< _output_get 0.0)
    (Variables|Default|Sethealth (+ (Variables|Default|Getarmor) (Variables|Default|Gethealth)))
    (Variables|Default|Setarmor 0.0) ; 盔甲值归零
  )
  (bind _returnvalue (UserInterface|CreateWidget "/Game/Zombies/BluePrints/DamageVignette.DamageVignette_C" (Game|GetPlayerController 0))) ; 伤害效果
  (UserInterface|Viewport|AddtoViewport _returnvalue 0))